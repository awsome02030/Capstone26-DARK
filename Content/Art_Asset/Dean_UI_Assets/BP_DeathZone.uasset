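; BP_DeathZone is a box trigger that turns on death-zone effects for a DARKCharacter who enters it.
; After a delay following overlap, it flags the character as in the death zone and raises its oxygen drain multiplier.
; It spawns an ExponentialHeightFog, then the FogUp timeline raises the fog found by GetActorOfClass, not necessarily the spawned one, toward a fixed height.
; Nothing reverses these effects on exit.
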(event `self.Box.OnComponentBeginOverlap`
  (params (OverlappedComponent :type "PrimitiveComponent Object Reference") (OtherActor :type "Actor Object Reference") (OtherComp :type "PrimitiveComponent Object Reference") (OtherBodyIndex :type Integer) (bFromSweep :type Boolean) (SweepResult :type "HitResult Structure (by ref)"))
  (bind _asdarkcharacter (cast `DARKCharacter` OtherActor))
  (`KismetSystemLibrary.Delay` 15.0)
  (set `DARKCharacter.bIsInDeathZone` true _asdarkcharacter)
  (set `DARKCharacter.OxygenDrainMultiplier` 20.0 _asdarkcharacter)
  (`|SpawnActorFromClass` "/Script/Engine.ExponentialHeightFog" (`KismetMathLibrary.Conv_VectorToTransform` (`SceneComponent.RelativeLocation` (`self.Box`))) "Undefined" "MultiplyWithRoot" null null)
  (bind _returnvalue (`GameplayStatics.GetActorOfClass` "/Script/Engine.ExponentialHeightFog"))
  (bind (_direction _alpha) (`Timeline|FogUp`)
    (:`Update`
      (`self.K2_SetActorLocation` _returnvalue (`KismetMathLibrary.MakeVector` (.x (`self.K2_GetActorLocation` _returnvalue)) (.y (`self.K2_GetActorLocation` _returnvalue)) (`KismetMathLibrary.Lerp` (.z (`self.K2_GetActorLocation` _returnvalue)) 15300.0 _alpha)) false false))))

(fn `UserConstructionScript`)