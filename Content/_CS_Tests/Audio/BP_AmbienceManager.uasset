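; Ambience manager Blueprint that plays background ambience and crossfades between sounds when the ambience changes.
; On BeginPlay it switches to a default ambience if no current one is set.
; ChangeAmbience ignores invalid or already-active sounds, then alternates between two audio components, fading the old one out while the new one fades in over a shared duration.
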(event `self.ReceiveBeginPlay`
  (`/Engine/EditorBlueprintResources/StandardMacros.IsValid` (`self.CurrentAmbience`)
    (:`Is Not Valid`
      (`self.ChangeAmbience` (`self.DefaultAmbience`)))))

(fn `ChangeAmbience`
  (params (NewAmbience :type "SoundBase Object Reference"))
  (bind _fadeduration (`self.FadeDuration`))
  (bind _ambience_a (`self.Ambience_A`))
  (bind _fadeduration_2 (`self.FadeDuration`))
  (bind _ambience_b (`self.Ambience_B`))
  (`/Engine/EditorBlueprintResources/StandardMacros.IsValid` NewAmbience
    (:`Is Valid`
      (if (not (== NewAmbience (`self.CurrentAmbience`)))
        (set `self.CurrentAmbience` NewAmbience)
        (if (`self.B_Using_A`)
          (`AudioComponent.Stop` _ambience_b)
          (`AudioComponent.SetSound` _ambience_b (`local.NewAmbience`))
          (`AudioComponent.FadeOut` (`self.Ambience_A`) _fadeduration_2 0.0 "Linear")
          (`AudioComponent.FadeIn` _ambience_b _fadeduration_2 1.0 0.0 "Linear")
          (set `self.B_Using_A` false)
          (else
            (`AudioComponent.Stop` _ambience_a)
            (`AudioComponent.SetSound` _ambience_a (`local.NewAmbience`))
            (`AudioComponent.FadeOut` (`self.Ambience_B`) _fadeduration 0.0 "Linear")
            (`AudioComponent.FadeIn` _ambience_a _fadeduration 1.0 0.0 "Linear")
            (set `self.B_Using_A` true)))))))

(fn `UserConstructionScript`)