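; Four-plate pressure puzzle that ends both cargo maintenance timers, normal and looped, once the player has pressed every plate.
; Each box overlap by BP_DARKCharacter increments a counter, destroys its trigger and lowers that plate by timeline, using start/end variables shared across plates.
; A DoOnce on timeline update plays sounds, lights the plate and, at four presses, calls CargoTimerFinished and clears the timers on cargo actors found at BeginPlay.
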(event `self.ReceiveBeginPlay`
  (bind _returnvalue (`GameplayStatics.GetActorOfClass` "/Game/_CS_Tests/RBP_CargoMaintenance.RBP_CargoMaintenance_C"))
  (set `self.Cargo Ref` _returnvalue)
  (bind _returnvalue_2 (`GameplayStatics.GetActorOfClass` "/Game/_CS_Tests/RBP_CargoMaintenanceLooped.RBP_CargoMaintenanceLooped_C"))
  (set `self.Looped Cargo Ref` _returnvalue_2))

(event `self.Box1.OnComponentBeginOverlap`
  (params (OverlappedComponent :type "PrimitiveComponent Object Reference") (OtherActor :type "Actor Object Reference") (OtherComp :type "PrimitiveComponent Object Reference") (OtherBodyIndex :type Integer) (bFromSweep :type Boolean) (SweepResult :type "HitResult Structure (by ref)"))
  (bind _looped_cargo_ref (`self.Looped Cargo Ref`))
  (bind _cargo_ref (`self.Cargo Ref`))
  (bind _relativelocation (`SceneComponent.RelativeLocation` (`self.Plate_Top1`)))
  (cast `/Game/INV/BP_DARKCharacter` OtherActor)
  (set `self.PlatesPressed` (+ (`self.PlatesPressed`) 1))
  (`ActorComponent.K2_DestroyComponent` (`self.Box1`))
  (bind _output_get (set `self.StartLocation` _relativelocation))
  (bind _output_get_2 (set `self.EndLocation` (+ _relativelocation (0.0 0.0 -10.0))))
  (bind (_direction _platemovement) (`Timeline|PlateAnim1`)
    (:`Update`
      (`SceneComponent.K2_SetRelativeLocation` (`self.Plate_Top1`) (`KismetMathLibrary.VLerp` _output_get _output_get_2 _platemovement) false false)
      (`/Engine/EditorBlueprintResources/StandardMacros.DoOnce` false
        (:`Completed`
          (`GameplayStatics.PlaySound2D` "/Game/Sounds/PressurePlateClick.PressurePlateClick" 1.0 1.0 0.0 null null)
          (`GameplayStatics.PlaySound2D` "/Game/Sounds/MachineMove_Fast.MachineMove_Fast" 1.0 1.0 0.0 null null)
          (`PrimitiveComponent.SetMaterial` (`self.Plate_Top1`) 0 "/Game/_CS_Tests/Materials/M_CargoPlatesOn.M_CargoPlatesOn")
          (if (== (`self.PlatesPressed`) 4)
            (`/Game/_CS_Tests/RBP_CargoMaintenance.CargoTimerFinished` _cargo_ref)
            (`KismetSystemLibrary.K2_ClearAndInvalidateTimerHandle` (`/Game/_CS_Tests/RBP_CargoMaintenance.Cargo Timer Handle` _cargo_ref))
            (`/Game/_CS_Tests/RBP_CargoMaintenanceLooped.CargoTimerFinished` _looped_cargo_ref)
            (`KismetSystemLibrary.K2_ClearAndInvalidateTimerHandle` (`/Game/_CS_Tests/RBP_CargoMaintenanceLooped.Cargo Timer Handle` _looped_cargo_ref))))))
    (:`Finished`
      (`PrimitiveComponent.SetMaterial` (`self.Plate_Bot1`) 0 "/Game/_CS_Tests/Materials/M_CargoPlatesOn.M_CargoPlatesOn"))))

(event `self.Box2.OnComponentBeginOverlap`
  (params (OverlappedComponent :type "PrimitiveComponent Object Reference") (OtherActor :type "Actor Object Reference") (OtherComp :type "PrimitiveComponent Object Reference") (OtherBodyIndex :type Integer) (bFromSweep :type Boolean) (SweepResult :type "HitResult Structure (by ref)"))
  (bind _cargo_ref (`self.Cargo Ref`))
  (bind _looped_cargo_ref (`self.Looped Cargo Ref`))
  (bind _relativelocation (`SceneComponent.RelativeLocation` (`self.Plate_Top2`)))
  (cast `/Game/INV/BP_DARKCharacter` OtherActor)
  (set `self.PlatesPressed` (+ (`self.PlatesPressed`) 1))
  (`ActorComponent.K2_DestroyComponent` (`self.Box2`))
  (bind _output_get (set `self.StartLocation` _relativelocation))
  (bind _output_get_2 (set `self.EndLocation` (+ _relativelocation (0.0 0.0 -10.0))))
  (bind (_direction _platemovement) (`Timeline|PlateAnim2`)
    (:`Update`
      (`SceneComponent.K2_SetRelativeLocation` (`self.Plate_Top2`) (`KismetMathLibrary.VLerp` _output_get _output_get_2 _platemovement) false false)
      (`/Engine/EditorBlueprintResources/StandardMacros.DoOnce` false
        (:`Completed`
          (`GameplayStatics.PlaySound2D` "/Game/Sounds/PressurePlateClick.PressurePlateClick" 1.0 1.0 0.0 null null)
          (`GameplayStatics.PlaySound2D` "/Game/Sounds/MachineMove_Fast.MachineMove_Fast" 1.0 1.0 0.0 null null)
          (`PrimitiveComponent.SetMaterial` (`self.Plate_Top2`) 0 "/Game/_CS_Tests/Materials/M_CargoPlatesOn.M_CargoPlatesOn")
          (if (== (`self.PlatesPressed`) 4)
            (`/Game/_CS_Tests/RBP_CargoMaintenance.CargoTimerFinished` _cargo_ref)
            (`KismetSystemLibrary.K2_ClearAndInvalidateTimerHandle` (`/Game/_CS_Tests/RBP_CargoMaintenance.Cargo Timer Handle` _cargo_ref))
            (`/Game/_CS_Tests/RBP_CargoMaintenanceLooped.CargoTimerFinished` _looped_cargo_ref)
            (`KismetSystemLibrary.K2_ClearAndInvalidateTimerHandle` (`/Game/_CS_Tests/RBP_CargoMaintenanceLooped.Cargo Timer Handle` _looped_cargo_ref))))))
    (:`Finished`
      (`PrimitiveComponent.SetMaterial` (`self.Plate_Bot2`) 0 "/Game/_CS_Tests/Materials/M_CargoPlatesOn.M_CargoPlatesOn"))))

(event `self.Box3.OnComponentBeginOverlap`
  (params (OverlappedComponent :type "PrimitiveComponent Object Reference") (OtherActor :type "Actor Object Reference") (OtherComp :type "PrimitiveComponent Object Reference") (OtherBodyIndex :type Integer) (bFromSweep :type Boolean) (SweepResult :type "HitResult Structure (by ref)"))
  (bind _cargo_ref (`self.Cargo Ref`))
  (bind _looped_cargo_ref (`self.Looped Cargo Ref`))
  (bind _relativelocation (`SceneComponent.RelativeLocation` (`self.Plate_Top3`)))
  (cast `/Game/INV/BP_DARKCharacter` OtherActor)
  (set `self.PlatesPressed` (+ (`self.PlatesPressed`) 1))
  (`ActorComponent.K2_DestroyComponent` (`self.Box3`))
  (bind _output_get (set `self.StartLocation` _relativelocation))
  (bind _output_get_2 (set `self.EndLocation` (+ _relativelocation (0.0 0.0 -10.0))))
  (bind (_direction _platemovement) (`Timeline|PlateAnim3`)
    (:`Update`
      (`SceneComponent.K2_SetRelativeLocation` (`self.Plate_Top3`) (`KismetMathLibrary.VLerp` _output_get _output_get_2 _platemovement) false false)
      (`/Engine/EditorBlueprintResources/StandardMacros.DoOnce` false
        (:`Completed`
          (`GameplayStatics.PlaySound2D` "/Game/Sounds/PressurePlateClick.PressurePlateClick" 1.0 1.0 0.0 null null)
          (`GameplayStatics.PlaySound2D` "/Game/Sounds/MachineMove_Fast.MachineMove_Fast" 1.0 1.0 0.0 null null)
          (`PrimitiveComponent.SetMaterial` (`self.Plate_Top3`) 0 "/Game/_CS_Tests/Materials/M_CargoPlatesOn.M_CargoPlatesOn")
          (if (== (`self.PlatesPressed`) 4)
            (`/Game/_CS_Tests/RBP_CargoMaintenance.CargoTimerFinished` _cargo_ref)
            (`KismetSystemLibrary.K2_ClearAndInvalidateTimerHandle` (`/Game/_CS_Tests/RBP_CargoMaintenance.Cargo Timer Handle` _cargo_ref))
            (`/Game/_CS_Tests/RBP_CargoMaintenanceLooped.CargoTimerFinished` _looped_cargo_ref)
            (`KismetSystemLibrary.K2_ClearAndInvalidateTimerHandle` (`/Game/_CS_Tests/RBP_CargoMaintenanceLooped.Cargo Timer Handle` _looped_cargo_ref))))))
    (:`Finished`
      (`PrimitiveComponent.SetMaterial` (`self.Plate_Bot3`) 0 "/Game/_CS_Tests/Materials/M_CargoPlatesOn.M_CargoPlatesOn"))))

(event `self.Box4.OnComponentBeginOverlap`
  (params (OverlappedComponent :type "PrimitiveComponent Object Reference") (OtherActor :type "Actor Object Reference") (OtherComp :type "PrimitiveComponent Object Reference") (OtherBodyIndex :type Integer) (bFromSweep :type Boolean) (SweepResult :type "HitResult Structure (by ref)"))
  (bind _looped_cargo_ref (`self.Looped Cargo Ref`))
  (bind _cargo_ref (`self.Cargo Ref`))
  (bind _relativelocation (`SceneComponent.RelativeLocation` (`self.Plate_Top4`)))
  (cast `/Game/INV/BP_DARKCharacter` OtherActor)
  (set `self.PlatesPressed` (+ (`self.PlatesPressed`) 1))
  (`ActorComponent.K2_DestroyComponent` (`self.Box4`))
  (bind _output_get (set `self.StartLocation` _relativelocation))
  (bind _output_get_2 (set `self.EndLocation` (+ _relativelocation (0.0 0.0 -10.0))))
  (bind (_direction _platemovement) (`Timeline|PlateAnim4`)
    (:`Update`
      (`SceneComponent.K2_SetRelativeLocation` (`self.Plate_Top4`) (`KismetMathLibrary.VLerp` _output_get _output_get_2 _platemovement) false false)
      (`/Engine/EditorBlueprintResources/StandardMacros.DoOnce` false
        (:`Completed`
          (`GameplayStatics.PlaySound2D` "/Game/Sounds/PressurePlateClick.PressurePlateClick" 1.0 1.0 0.0 null null)
          (`GameplayStatics.PlaySound2D` "/Game/Sounds/MachineMove_Fast.MachineMove_Fast" 1.0 1.0 0.0 null null)
          (`PrimitiveComponent.SetMaterial` (`self.Plate_Top4`) 0 "/Game/_CS_Tests/Materials/M_CargoPlatesOn.M_CargoPlatesOn")
          (if (== (`self.PlatesPressed`) 4)
            (`/Game/_CS_Tests/RBP_CargoMaintenance.CargoTimerFinished` _cargo_ref)
            (`KismetSystemLibrary.K2_ClearAndInvalidateTimerHandle` (`/Game/_CS_Tests/RBP_CargoMaintenance.Cargo Timer Handle` _cargo_ref))
            (`/Game/_CS_Tests/RBP_CargoMaintenanceLooped.CargoTimerFinished` _looped_cargo_ref)
            (`KismetSystemLibrary.K2_ClearAndInvalidateTimerHandle` (`/Game/_CS_Tests/RBP_CargoMaintenanceLooped.Cargo Timer Handle` _looped_cargo_ref))))))
    (:`Finished`
      (`PrimitiveComponent.SetMaterial` (`self.Plate_Bot4`) 0 "/Game/_CS_Tests/Materials/M_CargoPlatesOn.M_CargoPlatesOn"))))

(fn `UserConstructionScript`)