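; Haunt button test actor that takes over the player's view during interaction and signals when its completion requirement is met.
; Beginning interaction stops and locks movement, then a timeline lerps the control rotation along the shortest path toward ButtonFocusPoint.
; Ending interaction releases the movement lock.
; When the remaining completion count reaches zero, it plays a correct sound and swaps a mesh material to green glow.
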(event `self.OnCompleteNeededChanged`
  (params (NewCompleteNeeded :type Integer))
  (if (== NewCompleteNeeded 0)
    (`GameplayStatics.PlaySound2D` "/Game/Sounds/Correct.Correct" 1.0 1.0 0.0 null null)
    (`PrimitiveComponent.SetMaterial` (`self.StaticMeshComponent`) 1 "/Game/_CS_Tests/Materials/Capsule/M_GreenGlow.M_GreenGlow")))

(event `Begin Button Interaction`
  (bind _returnvalue (`GameplayStatics.GetPlayerController` 0))
  (`MovementComponent.StopMovementImmediately` (`Character.CharacterMovement` (`GameplayStatics.GetPlayerCharacter` 0)))
  (`Controller.SetIgnoreMoveInput` _returnvalue true)
  (set `self.Look Start Location` (`Controller.GetControlRotation` _returnvalue))
  (set `self.Look Target Location` (`KismetMathLibrary.FindLookAtRotation` (`PlayerCameraManager.GetCameraLocation` (`GameplayStatics.GetPlayerCameraManager` 0)) (`SceneComponent.K2_GetComponentLocation` (`self.ButtonFocusPoint`))))
  (bind (_direction _lookat) (`Timeline|Timeline`)
    (:`Update`
      (`Controller.SetControlRotation` _returnvalue (`KismetMathLibrary.RLerp` (`self.Look Start Location`) (`self.Look Target Location`) _lookat true)))))

(event `End Button Interaction`
  (`Controller.ResetIgnoreMoveInput` (`GameplayStatics.GetPlayerController` 0)))

(fn `UserConstructionScript`)