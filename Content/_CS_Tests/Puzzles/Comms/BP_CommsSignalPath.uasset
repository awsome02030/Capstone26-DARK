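; Comms puzzle signal path that shows a timed pulse along a configurable set of wire meshes.
; PlayPulse restarts a timer and swaps every valid wire to the pulsing material, while StopPulse clears the timer and restores the normal one.
; ConfigureWires stops any pulse before replacing the mesh set.
; FinishPulse prints a debug message and, if still pulsing, stops and fires OnPulseFinished.
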(event `Play Pulse`
  (`KismetSystemLibrary.K2_ClearAndInvalidateTimerHandle` (`self.PulseTimerHandle`))
  (set `self.IsPulsing` true)
  (`self.ApplyWireMaterial`)
  (bind _returnvalue (`KismetSystemLibrary.K2_SetTimerDelegate` (`|CreateDelegate` :!event `FinishPulse`) (`self.PulseDuration`)))
  (set `self.PulseTimerHandle` _returnvalue))

(event `Stop Pulse`
  (set `self.IsPulsing` false)
  (`KismetSystemLibrary.K2_ClearAndInvalidateTimerHandle` (`self.PulseTimerHandle`))
  (`self.ApplyWireMaterial`))

(fn `ApplyWireMaterial`
  (for _array_element (`self.WireMeshes`)
    (`/Engine/EditorBlueprintResources/StandardMacros.IsValid` _array_element
      (:`Is Valid`
        (if (`self.IsPulsing`)
          (`PrimitiveComponent.SetMaterial` _array_element 0 "/Game/_CS_Tests/Materials/M_WiresPulsing.M_WiresPulsing")
          (else
            (`PrimitiveComponent.SetMaterial` _array_element 0 "/Game/_CS_Tests/Materials/M_Wires.M_Wires"))))))
  (return))

(fn `ConfigureWires`
  (params (NewWireMeshes :type "Array of StaticMeshComponent Object Reference"))
  (`self.Stop Pulse`)
  (set `self.WireMeshes` NewWireMeshes)
  (`self.ApplyWireMaterial`))

(fn `FinishPulse`
  (`KismetSystemLibrary.PrintString` "PULSE FINISHED" true true (struct :`G` 0.66 :`B` 1.0 :`A` 1.0) 10.0)
  (if (`self.IsPulsing`)
    (`self.Stop Pulse`)
    (`self.OnPulseFinished` self)
    (else
      (return))))

(fn `UserConstructionScript`)