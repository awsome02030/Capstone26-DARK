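; Puzzle fuse box actor that shows a fuse sliding into place and turns its indicator light green when OnFuseInserted fires.
; The event plays a click, reveals the fuse mesh and starts a timeline fading a dynamic light material and point light from white to green.
; Once inserted, Tick eases the fuse toward an end position offset along local X, computed at BeginPlay.
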(event `self.ReceiveBeginPlay`
  (set `self.FuseEnd` (- (`SceneComponent.RelativeLocation` (`self.SM_Power_Fuse`)) (100.0 0.0 0.0)))
  (bind _returnvalue (`PrimitiveComponent.CreateDynamicMaterialInstance` (`self.SM_HauntLight`) 1 "/Game/_CS_Tests/Materials/M_FuseBoxLight.M_FuseBoxLight" "None"))
  (set `self.Light Material` _returnvalue))

(event `self.OnFuseInserted`
  (`GameplayStatics.PlaySound2D` "/Game/Sounds/PressurePlateClick.PressurePlateClick" 1.0 1.0 0.0 null null)
  (`SceneComponent.SetVisibility` (`self.SM_Power_Fuse`) true true)
  (set `self.Inserted` true)
  (bind (_direction _color_change) (`Timeline|Fade To Green` :!via `PlayFromStart`)
    (:`Update`
      (bind _returnvalue (`KismetMathLibrary.LinearColorLerp` (struct :`R` 1.0 :`G` 1.0 :`B` 1.0 :`A` 1.0) (struct :`G` 1.0 :`B` 0.222 :`A` 1.0) _color_change))
      (`MaterialInstanceDynamic.SetVectorParameterValue` (`self.Light Material`) "Light Color" _returnvalue)
      (`LightComponent.SetLightColor` (`self.PointLight`) _returnvalue true))))

(event `self.ReceiveTick`
  (params (DeltaSeconds :type "Float (single-precision)"))
  (if (`self.Inserted`)
    (`SceneComponent.K2_SetRelativeLocation` (`self.SM_Power_Fuse`) (`KismetMathLibrary.VInterpTo` (`SceneComponent.RelativeLocation` (`self.SM_Power_Fuse`)) (`self.FuseEnd`) (`GameplayStatics.GetWorldDeltaSeconds`) 3.0) false false)))

(fn `UserConstructionScript`)