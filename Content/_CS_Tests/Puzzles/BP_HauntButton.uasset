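; BP_HauntButton is a puzzle button that tracks entering batteries into wall sockets and reflects that progress in its material and the HUD task text.
; When the needed count changes it updates WBP_HUD; at zero it plays a sound, shows the ready material, then after a delay shows the escape-the-Entity objective.
; Tick polls GridManager and switches to the off material once the escape pod room has spawned.
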(event `self.OnCompleteNeededChanged`
  (params (NewCompleteNeeded :type Integer))
  (bind _foundwidgets (`WidgetBlueprintLibrary.GetAllWidgetsOfClass` "/Game/UI/WidgetBlueprints/WBP_HUD.WBP_HUD_C"))
  (for _array_element _foundwidgets
    _)
  (if (== NewCompleteNeeded 0)
    (`GameplayStatics.PlaySound2D` "/Game/Sounds/Correct.Correct" 1.0 1.0 0.0 null null)
    (`PrimitiveComponent.SetMaterial` (`self.StaticMeshComponent`) 1 "/Game/_CS_Tests/Materials/M_HauntButtonReady.M_HauntButtonReady")
    (`/Game/UI/WidgetBlueprints/WBP_HUD.SetTaskNotification` _array_element "Enter batteries into wall sockets (2/2)" false)
    (`KismetSystemLibrary.Delay` 1.5)
    (`/Game/UI/WidgetBlueprints/WBP_HUD.SetTaskNotification` _array_element "Escape the Entity" true)
    (else
      (`/Game/UI/WidgetBlueprints/WBP_HUD.SetTaskNotification` _array_element "Enter batteries into wall sockets (1/2)" false))))

(event `self.ReceiveTick`
  (params (DeltaSeconds :type "Float (single-precision)"))
  (bind _returnvalue (`GameplayStatics.GetActorOfClass` "/Script/DARK.GridManager"))
  (if (`GridManager.bEscapePodRoomSpawned` _returnvalue)
    (`PrimitiveComponent.SetMaterial` (`self.StaticMeshComponent`) 1 "/Game/_CS_Tests/Materials/M_HauntButtonOff.M_HauntButtonOff")))

(fn `UserConstructionScript`)