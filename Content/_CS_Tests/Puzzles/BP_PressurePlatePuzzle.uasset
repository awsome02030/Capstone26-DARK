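; BP_PressurePlatePuzzle is a four-plate pressure puzzle that tracks progress on a "Stabilize Cargo" task.
; On BeginPlay it binds to the press dispatcher of four child-actor BP_PressurePlate instances.
; Each press increments a counter, never decremented here, and updates the task notification on the first WBP_HUD found.
; When the count reaches four, a DoOnce-guarded call broadcasts OnAllPlatesPressed.
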(event `self.ReceiveBeginPlay`
  (for _array_element (`|MakeArray` (`self.BP_PressurePlate1`) (`self.BP_PressurePlate2`) (`self.BP_PressurePlate3`) (`self.BP_PressurePlate4`))
    (bind _asbp_pressure_plate (cast `/Game/_CS_Tests/Puzzles/BP_PressurePlate` (`ChildActorComponent.ChildActor` _array_element)))
    (add `/Game/_CS_Tests/Puzzles/BP_PressurePlate.OnPlatePressed` _asbp_pressure_plate (delegate `Handle Plates Pressed`))))

(event `Handle Plates Pressed`
  (bind _output_get (set `self.PlatesPressed` (+ (`self.PlatesPressed`) 1)))
  (`|ExecutionSequence`
    (:`then_0`
      (bind _foundwidgets (`WidgetBlueprintLibrary.GetAllWidgetsOfClass` "/Game/UI/WidgetBlueprints/WBP_HUD.WBP_HUD_C" false))
      (bind _output (`|GetArrayItem` _foundwidgets))
      (`/Engine/EditorBlueprintResources/StandardMacros.IsValid` _output
        (:`Is Valid`
          (`/Game/UI/WidgetBlueprints/WBP_HUD.SetTaskNotification` _output (`|FormatText` "Stabilize Cargo ({Count}/4)" (`self.PlatesPressed`)) false))))
    (:`then_1`
      (if (== _output_get 4)
        (`/Engine/EditorBlueprintResources/StandardMacros.DoOnce` false
          (:`Completed`
            (`self.On All Plates Pressed`)))))))

(fn `UserConstructionScript`)