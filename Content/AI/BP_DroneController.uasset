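; AI controller for a drone that drives its behavior tree and switches between search and hunt states.
; On possess it waits briefly, runs BT_Drone and enters the search state.
; Helper functions write the state, target player and last known location to the Blackboard.
; CanSeeActor checks the perception component's last sensed stimuli and returns whether the sight sense currently detects the actor.
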(event `self.ReceivePossess`
  (params (PossessedPawn :type "Pawn Object Reference"))
  (`KismetSystemLibrary.Delay` 0.2)
  (`self.RunBehaviorTree` "/Game/AI/BT_Drone.BT_Drone")
  (`self.SetSearchState`))

(fn `CanSeeActor`
  (params (Actor :type "Actor Object Reference"))
  (returns (Sensed :type Boolean))
  (bind _info (`AIPerceptionComponent.GetActorsPerception` (`self.AIPerception`) Actor))
  (for _array_element (`.LastSensedStimuli` (break `ActorPerceptionBlueprintInfo` _info))
    (bind _returnvalue (`AIPerceptionSystem.GetSenseClassForStimulus` _array_element))
    (if (== _returnvalue "/Script/AIModule.AISense_Sight")
      (return (`.bSuccessfullySensed` (break `AIStimulus` _array_element))))))

(fn `SetHuntState`
  (params (Player :type "Actor Object Reference"))
  (bind _blackboard (`self.Blackboard`))
  (`BlackboardComponent.SetValueAsObject` _blackboard (`self.Player`) Player)
  (`BlackboardComponent.SetValueAsEnum` _blackboard (`self.State`) (enumliteral `/Game/AI/E_AI_States` "NewEnumerator1")))

(fn `SetLastKnownLocation`
  (params (LastKnownLocation :type "Vector Structure"))
  (`BlackboardComponent.SetValueAsVector` (`self.Blackboard`) (`self.LastKnownLocation`) LastKnownLocation))

(fn `SetSearchState`
  (`BlackboardComponent.SetValueAsEnum` (`self.Blackboard`) (`self.State`) (enumliteral `/Game/AI/E_AI_States` "NewEnumerator0")))

(fn `UserConstructionScript`)