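; BP_EnemySearchPath is a spline-based patrol path that supplies world-space waypoints, apparently for enemy AI.
; The Patrol event advances PatrolIndex and resets it to zero upon reaching the last spline point's index, so that final point is skipped.
; GetSplinePointAsWorldPosition returns the world location of the spline point at the current index.
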(event `Patrol`
  (bind _output_get (set `self.PatrolIndex` (+ (`self.PatrolIndex`) 1)))
  (if (== _output_get (- (`SplineComponent.GetNumberOfSplinePoints` (`self.Spline`)) 1))
    (set `self.PatrolIndex` 0)))

(fn `GetSplinePointAsWorldPosition`
  (returns (Location :type "Vector Structure"))
  (return (`SplineComponent.GetLocationAtSplinePoint` (`self.Spline`) (`self.PatrolIndex`) "World")))

(fn `UserConstructionScript`)