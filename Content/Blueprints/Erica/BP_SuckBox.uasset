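; BP_SuckBox is an actor that gets pulled to a target location when its StartSuck event is called.
; StartSuck stores the target and raises a moving flag, and Tick then eases the actor toward it with VInterpTo at MoveSpeed, without sweeping.
; Within a small distance it snaps onto the target and stops.
; BeginPlay caches the starting scale, which the graph never uses.
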(event `self.ReceiveBeginPlay`
  (set `self.StartScale` (`self.GetActorScale3D`)))

(event `StartSuck`
  (params (`New TargetLocation` :type "Vector Structure"))
  (set `self.TargetLocation` `New TargetLocation`)
  (set `self.bIsMoving` true))

(event `self.ReceiveTick`
  (params (DeltaSeconds :type "Float (single-precision)"))
  (bind _targetlocation (`self.TargetLocation`))
  (if (`self.bIsMoving`)
    (`self.K2_SetActorLocation` (`KismetMathLibrary.VInterpTo` (`self.K2_GetActorLocation`) (`self.TargetLocation`) (`GameplayStatics.GetWorldDeltaSeconds`) (`self.MoveSpeed`)))
    (if (<= (`KismetMathLibrary.VSize` (- (`self.K2_GetActorLocation`) _targetlocation)) 10.0)
      (`self.K2_SetActorLocation` _targetlocation)
      (set `self.bIsMoving` false))))

(fn `UserConstructionScript`)