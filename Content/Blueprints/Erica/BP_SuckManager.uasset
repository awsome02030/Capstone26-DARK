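; Manager that pulls every BP_SuckBox in the level toward a target actor when Cargo_trigger is overlapped.
; On overlap it gathers all the boxes and starts the sequence after a short delay.
; A self-calling MoveNextBox event walks the array with a brief delay between steps, passing the target's location to each box's StartSuck for a staggered effect.
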(event `self.cargo_trigger.OnActorBeginOverlap`
  (params (OverlappedActor :type "Actor Object Reference") (OtherActor :type "Actor Object Reference"))
  (bind _outactors (`GameplayStatics.GetAllActorsOfClass` "/Game/Blueprints/Erica/BP_SuckBox.BP_SuckBox_C"))
  (set `self.Boxes` _outactors)
  (`KismetSystemLibrary.Delay` 0.5)
  (`self.StartSuckingBoxes`))

(event `StartSuckingBoxes`
  (set `self.CurrentIndex` 0)
  (`self.MoveNextBox`))

(event `MoveNextBox`
  (if (< (`self.CurrentIndex`) (`KismetArrayLibrary.Array_Length` (`self.Boxes`)))
    (`/Game/Blueprints/Erica/BP_SuckBox.StartSuck` (`|GetArrayItem` (`self.Boxes`) (`self.CurrentIndex`)) (`self.K2_GetActorLocation` (`self.TargetActor`)))
    (set `self.CurrentIndex` (+ (`self.CurrentIndex`) 1))
    (`KismetSystemLibrary.Delay` 0.2)
    (`self.MoveNextBox`)))

(fn `UserConstructionScript`)