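; Automatic double sliding door for the cargo room that opens when the first-person character enters its trigger and closes when they leave.
; After a short delay, begin overlap plays the OpenCloseDoor timeline from the start, while end overlap reverses a separate timeline from the end.
; Each timeline's DoorTrack lerps the left and right panels' relative X location in opposite directions.
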(event `self.Open_Trigger.OnActorBeginOverlap`
  (params (OverlappedActor :type "Actor Object Reference") (OtherActor :type "Actor Object Reference"))
  (cast `/Game/FirstPerson/Blueprints/BP_FirstPersonCharacter` OtherActor)
  (`KismetSystemLibrary.Delay` 0.5)
  (bind (_direction _door_track) (`Timeline|Open/Close Door` :!via `PlayFromStart`)
    (:`Update`
      (`SceneComponent.K2_SetRelativeLocation` (`self.Door_Left`) (`KismetMathLibrary.MakeVector` (`KismetMathLibrary.Lerp` 0.0 100.0 _door_track)) false false)
      (`SceneComponent.K2_SetRelativeLocation` (`self.Door_Right`) (`KismetMathLibrary.MakeVector` (`KismetMathLibrary.Lerp` 0.0 -100.0 _door_track)) false false))))

(event `self.Open_Trigger.OnActorEndOverlap`
  (params (OverlappedActor :type "Actor Object Reference") (OtherActor :type "Actor Object Reference"))
  (cast `/Game/FirstPerson/Blueprints/BP_FirstPersonCharacter` OtherActor)
  (`KismetSystemLibrary.Delay` 0.5)
  (bind (_direction _door_track) (`Timeline|Timeline` :!via `ReverseFromEnd`)
    (:`Update`
      (`SceneComponent.K2_SetRelativeLocation` (`self.Door_Left`) (`KismetMathLibrary.MakeVector` (`KismetMathLibrary.Lerp` 0.0 100.0 _door_track)) false false)
      (`SceneComponent.K2_SetRelativeLocation` (`self.Door_Right`) (`KismetMathLibrary.MakeVector` (`KismetMathLibrary.Lerp` 0.0 -100.0 _door_track)) false false))))

(fn `UserConstructionScript`)