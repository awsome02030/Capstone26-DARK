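; BP_Cargo_Dead is a hazard zone that drains a DARKCharacter's oxygen while it overlaps the Cargo_trigger actor.
; Entering stores the character and starts a looping timer, if none is active, that repeatedly calls DrainOxygen to reduce oxygen by a fixed amount.
; The timer is cleared and the stored character released when oxygen runs out or a DARKCharacter leaves the trigger.
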(event `self.Cargo_trigger.OnActorBeginOverlap`
  (params (OverlappedActor :type "Actor Object Reference") (OtherActor :type "Actor Object Reference"))
  (bind _asdarkcharacter (cast `DARKCharacter` OtherActor))
  (set `self.Player` _asdarkcharacter)
  (if (not (`KismetSystemLibrary.K2_IsTimerActiveHandle` (`self.DrainTimerHandle`)))
    (bind _returnvalue (`KismetSystemLibrary.K2_SetTimerDelegate` (delegate `Drain Oxygen`) 0.2 true))
    (set `self.DrainTimerHandle` _returnvalue)))

(event `Drain Oxygen`
  (bind _player (`self.Player`))
  (`/Engine/EditorBlueprintResources/StandardMacros.IsValid` _player
    (:`Is Valid`
      (`DARKCharacter.ReduceOxygen` _player 5)
      (if (<= (`DARKCharacter.Oxygen` _player) 0)
        (`KismetSystemLibrary.K2_ClearAndInvalidateTimerHandle` (`self.DrainTimerHandle`))
        (set `self.Player` null)))))

(event `self.Cargo_trigger.OnActorEndOverlap`
  (params (OverlappedActor :type "Actor Object Reference") (OtherActor :type "Actor Object Reference"))
  (cast `DARKCharacter` OtherActor)
  (`KismetSystemLibrary.K2_ClearAndInvalidateTimerHandle` (`self.DrainTimerHandle`))
  (set `self.Player` null))

(fn `UserConstructionScript`)