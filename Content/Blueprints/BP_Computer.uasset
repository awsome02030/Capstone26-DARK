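; BP_Computer is a computer actor that brings up a password screen when the DARKCharacter overlaps its Box.
; A DoOnce gates the sequence, with the IsRespawned flag choosing whether an overlap resets or enters it.
; The sequence blocks player movement, look and input, creates WBP_Password, focuses it with the mouse cursor shown, and clears IsRespawned.
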(event `self.Box.OnComponentBeginOverlap`
  (params (OverlappedComponent :type "PrimitiveComponent Object Reference") (OtherActor :type "Actor Object Reference") (OtherComp :type "PrimitiveComponent Object Reference") (OtherBodyIndex :type Integer) (bFromSweep :type Boolean) (SweepResult :type "HitResult Structure (by ref)"))
  (bind _returnvalue (`GameplayStatics.GetPlayerController` 0))
  (bind _returnvalue_2 (`GameplayStatics.GetPlayerController` 0))
  (cast `DARKCharacter` OtherActor)
  (if (`self.IsRespawned`)
    (goto _label :!via `Reset`)
    (else
      (`/Engine/EditorBlueprintResources/StandardMacros.DoOnce` false :!label _label
        (:`Completed`
          (`Controller.SetIgnoreMoveInput` _returnvalue true)
          (`Controller.SetIgnoreLookInput` _returnvalue true)
          (bind _returnvalue_3 (`|CreateWidget` "/Game/UI/WidgetBlueprints/WBP_Password.WBP_Password_C"))
          (bind _output_get (set `self.Password` _returnvalue_3))
          (`UserWidget.AddToViewport` _output_get 0)
          (`WidgetBlueprintLibrary.SetInputMode_GameAndUIEx` _returnvalue_2 _output_get)
          (set `PlayerController.bShowMouseCursor` true _returnvalue_2)
          (`self.DisableInput` _returnvalue_2 _returnvalue_2)
          (set `self.IsRespawned` false))))))

(fn `UserConstructionScript`)