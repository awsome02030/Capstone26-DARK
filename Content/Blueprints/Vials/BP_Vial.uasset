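; BP_Vial is a colored vial that reports its breaking to the laboratory.
; On BeginPlay it finds the RBP_Laboratory and RBP_LaboratoryLooped actors and sets a glow material from VialColor, with Yellow using the green glow.
; Tick polls IsBroken, which is set outside these graphs, and registers the color once with the standard lab, falling back to the looped lab if that is invalid.
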(event `self.ReceiveBeginPlay`
  (bind _returnvalue (`GameplayStatics.GetActorOfClass` "/Game/_CS_Tests/Rooms/RBP_Laboratory.RBP_Laboratory_C"))
  (set `self.Lab Ref` _returnvalue)
  (bind _returnvalue_2 (`GameplayStatics.GetActorOfClass` "/Game/_CS_Tests/Rooms/RBP_LaboratoryLooped.RBP_LaboratoryLooped_C"))
  (set `self.Looped Lab Ref` _returnvalue_2)
  (`PrimitiveComponent.SetMaterial` (`self.VialMesh`) 1 (select `EVialColor` (`self.VialColor`) :`Red` "/Game/_CS_Tests/Materials/Capsule/M_RedGlow.M_RedGlow" :`Blue` "/Game/_CS_Tests/Materials/Capsule/M_BlueGlow.M_BlueGlow" :`Yellow` "/Game/_CS_Tests/Materials/Capsule/M_GreenGlow.M_GreenGlow" :!type "MaterialInterface Object Reference")))

(event `self.ReceiveTick`
  (params (DeltaSeconds :type "Float (single-precision)"))
  (bind _lab_ref (`self.Lab Ref`))
  (bind _looped_lab_ref (`self.Looped Lab Ref`))
  (if (`self.bIsBroken`)
    (if (not (`self.Is Registered?`))
      (`/Engine/EditorBlueprintResources/StandardMacros.IsValid` _lab_ref
        (:`Is Valid`
          (`/Game/_CS_Tests/Rooms/RBP_Laboratory.RegisterVialBreaking` _lab_ref (`self.VialColor`))
          (set `self.Is Registered?` true))
        (:`Is Not Valid`
          (`/Engine/EditorBlueprintResources/StandardMacros.IsValid` _looped_lab_ref
            (:`Is Valid`
              (`/Game/_CS_Tests/Rooms/RBP_LaboratoryLooped.RegisterVialBreaking` _looped_lab_ref (`self.VialColor`))
              (set `self.Is Registered?` true))))))))

(fn `UserConstructionScript`)