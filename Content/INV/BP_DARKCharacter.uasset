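; BP_DARKCharacter is the player character, handling audio logs with captions, crosshair and interact prompts, and a low-gravity toggle.
; PlayAudio runs a looping timer that feeds elapsed time to the caption widget until the sound ends.
; A per-tick camera trace gives WidgetInteraction a custom hit, letting interact click comms receiver screens.
; The intro log ending sets the escape pod task and unblocks the keypad; player reset resets the comms puzzle.
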(event OnAudioFinished(CurrentAudio)
  (bind _captionwidgetref (Variables|Default|GetCaptionWidgetRef))
  ;[0.15 0.15 0.15 0.5] Caption System
  (Utilities|Time|ClearandInvalidateTimerbyHandle (Variables|Default|GetCaptionTimerHandle))
  (Utilities|IsValid _captionwidgetref
    (:Is%20Valid
      (Default|HideCaption _captionwidgetref))))

(event Custom|PlayAudio
  (params (NewAudio :type Sound%20Base%20Object%20Reference))
  (bind _currentaudio (Variables|Default|GetCurrentAudio))
  ;[0.15 0.15 0.15 0.5] Play Audio
  (Utilities|Time|ClearandInvalidateTimerbyHandle (Variables|Default|GetCaptionTimerHandle))
  (Audio|Components|Audio|Stop _currentaudio)
  (Audio|Components|Audio|SetSound _currentaudio NewAudio)
  (Audio|Components|Audio|Play _currentaudio 0.0)
  (Variables|Default|SetAudioStartTime (Utilities|Time|GetGameTimeinSeconds))
  (bind _returnvalue (Utilities|Time|SetTimerbyEvent (EventDispatchers|CreateEvent :!event Custom|UpdateAudioCaption) 0.05 true))
  (Variables|Default|SetCaptionTimerHandle _returnvalue))

(event Custom|UpdateAudioCaption
  (bind _captionwidgetref (Variables|Default|GetCaptionWidgetRef))
  ;[0.15 0.15 0.15 0.5] Caption System
  (Utilities|IsValid _captionwidgetref
    (:Is%20Valid
      (Default|UpdateCaptionbyTime _captionwidgetref (- (Utilities|Time|GetGameTimeinSeconds) (Variables|Default|GetAudioStartTime))))))

(event Custom|Handle%20Log%20Finished
  ;[0.15 0.15 0.15 0.5] Handle Task After Intro Log End (NEEDS TO BE FIXED, OVERWRITES ROOM BECAUSE DIALOG TAKES TOO LONG)
  (if (Variables|Default|GetWaitingForIntroAudio)
    (Variables|Default|SetWaitingForIntroAudio false)
    (bind _foundwidgets (Widget|GetAllWidgetsOfClass "/Game/UI/WidgetBlueprints/WBP_HUD.WBP_HUD_C" true))
    (for _array_element _foundwidgets
      (Default|SetTaskNotification _array_element "Find Escape Pod Room" true)
      (Utilities|FlowControl|Delay 0.5)
      (bind _returnvalue (Actor|GetActorOfClass "/Game/_CS_Tests/Rooms/RBP_StartingRoom.RBP_StartingRoom_C"))
      (Default|DisableKeypadBlocker _returnvalue))))

(event Input|EnhancedActionEvents|EnhancedInputActionIA_Interact
  (params (ActionValue :type Boolean) (ElapsedSeconds :type Float%20%28double-precision%29) (TriggeredSeconds :type Float%20%28double-precision%29) (InputAction :type Input%20Action%20Object%20Reference :default "/Game/INV/IA_Interact.IA_Interact"))
  (bind _widgetinteraction (Variables|Default|GetWidgetInteraction))
  (bind _returnvalue (Class|WidgetInteractionComponent|GetHoveredWidgetComponent _widgetinteraction))
  ;[0.15 0.15 0.15 0.5] On Interact, get hovered widget and press key
  (:Started
    (Utilities|IsValid _returnvalue
      (:Is%20Valid
        (Utilities|Casting|CastToBP_CommsReceiver (Components|GetOwner _returnvalue))
        (if (Class|WidgetInteractionComponent|IsOverInteractableWidget (Variables|Default|GetWidgetInteraction))
          (Variables|Default|SetCommsPointerPressed true)
          (Class|WidgetInteractionComponent|PressPointerKey (Variables|Default|GetWidgetInteraction) "LeftMouseButton")))))
  (:Canceled
    (CallFunction|ReleaseCommsPointer :!label _label))
  (:Completed
    (goto _label)))

(event Input|EnhancedActionEvents|EnhancedInputActionIA_GravityChange
  (params (ActionValue :type Boolean) (ElapsedSeconds :type Float%20%28double-precision%29) (TriggeredSeconds :type Float%20%28double-precision%29) (InputAction :type Input%20Action%20Object%20Reference :default "/Game/INV/IA_GravityChange.IA_GravityChange"))
  ;[0.15 0.15 0.15 0.5] Gravity
  (:Started
    (if (== (Variables|/Script/Engine.CharacterMovementComponent|GetGravityScale (Variables|Character|GetCharacterMovement)) 1.0)
      (Variables|/Script/Engine.CharacterMovementComponent|SetGravityScale (Variables|Character|GetCharacterMovement) 0.1)
      (else
        (Variables|/Script/Engine.CharacterMovementComponent|SetGravityScale (Variables|Character|GetCharacterMovement) 1.0)))))

(event EventOnPlayerResetStarted
  (bind _active_comms_manager (Variables|Default|GetActive%20Comms%20Manager))
  ;[0.15 0.15 0.15 0.5] On Reset
  (Utilities|FlowControl|Sequence
    (:then_0
      (Utilities|IsValid _active_comms_manager
        (:Is%20Valid
          (Default|ResetPuzzle _active_comms_manager)
          (Utilities|FlowControl|Delay 3.0)
          (Audio|Components|Audio|Stop (Variables|Default|GetCurrentAudio)))))
    (:then_1
      (bind _foundwidgets (Widget|GetAllWidgetsOfClass "/Game/UI/WidgetBlueprints/WBP_HUD.WBP_HUD_C" true))
      (for _array_element _foundwidgets
        (Default|SetTaskNotification _array_element "No Current Task" true)))))

(event EventBeginPlay
  ;[0.15 0.15 0.15 0.5] Get Refs for Widgets
  (bind _output_get (Variables|Default|SetLogPlaybackComponent (Variables|Default|GetCurrentAudio)))
  (EventDispatchers|BindEventtoOnAudioFinished _output_get (delegate Custom|Handle%20Log%20Finished))
  (if (Pawn|IsLocallyControlled)
    (bind _returnvalue (UserInterface|CreateWidget "/Game/LanguageSystem/CaptionSystem/WBP_AudioCaption.WBP_AudioCaption_C" (Game|GetPlayerController 0)))
    (bind _output_get_2 (Variables|Default|SetCaptionWidgetRef _returnvalue))
    (UserInterface|Viewport|AddtoViewport _output_get_2 10)
    (bind _returnvalue_2 (UserInterface|CreateWidget "/Game/UI/WidgetBlueprints/WBP_Crosshair.WBP_Crosshair_C" (Game|GetPlayerController 0)))
    (bind _output_get_3 (Variables|Default|SetCrosshairRef _returnvalue_2))
    (UserInterface|Viewport|AddtoViewport _output_get_3 10)
    (Default|RefreshCrosshairVisibility _output_get_3)))

(event EventTick
  (params (DeltaSeconds :type Float%20%28single-precision%29))
  (bind _returnvalue (Game|GetPlayerCameraManager 0))
  (bind _returnvalue_2 (Camera|GetCameraLocation _returnvalue))
  ;[0.15 0.15 0.15 0.5] Get where player is looking for custom widget hit
  (bind _outhit (Collision|LineTraceByChannel _returnvalue_2 (+ _returnvalue_2 (* (Math|Vector|GetForwardVector (Camera|GetCameraRotation _returnvalue)) (Variables|Default|GetVectorMultiply))) "TraceTypeQuery1" true 0 "None"))
  (Class|WidgetInteractionComponent|SetCustomHitResult (Variables|Default|GetWidgetInteraction) _outhit))

(event EventUpdateInteractPrompt
  (params (Widget :type User%20Widget%20Object%20Reference) (bShowPrompt :type Boolean))
  ;[0.15 0.15 0.15 0.5] Update Interact Available
  (bind _aswbp_interact (Utilities|Casting|CastToWBP_Interact Widget))
  (Variables|Default|SetInteractRef _aswbp_interact)
  (Variables|Default|SetActorPromptRequested bShowPrompt)
  (CallFunction|RefreshInteractUI))

(event Input|KeyboardEvents|DebugKey5
  (params (Key :type Key%20Structure :default "None") (ActionValue :type Input%20Action%20Value%20Structure))
  (bind _logplaybackcomponent (Variables|Default|GetLogPlaybackComponent))
  (:Pressed
    (if (Variables|Default|GetWaitingForIntroAudio)
      (Utilities|IsValid _logplaybackcomponent
        (:Is%20Valid
          (Audio|Components|Audio|Stop _logplaybackcomponent))))))

(fn ConstructionScript)

(fn UpdateCaptionData
  (params (NewCues :type Array%20of%20ST%20Caption%20Cue%20Structures))
  (bind _captionwidgetref (Variables|Default|GetCaptionWidgetRef))
  (Utilities|IsValid _captionwidgetref
    (:Is%20Valid
      (Default|SetCaptionData _captionwidgetref NewCues))))

(fn ReleaseCommsPointer
  (if (Variables|Default|GetCommsPointerPressed)
    (Variables|Default|SetCommsPointerPressed false)
    (Class|WidgetInteractionComponent|ReleasePointerKey (Variables|Default|GetWidgetInteraction) "LeftMouseButton")))

(fn RefreshInteractUI
  (bind _crosshairref (Variables|Default|GetCrosshairRef))
  (bind _interactref (Variables|Default|GetInteractRef))
  (Utilities|IsValid _crosshairref
    (:Is%20Valid
      (LocalVariables|SetFinalInteractionVisible%20%28Local%29 (Math|Boolean|ANDBoolean (or (Variables|Default|GetActorPromptRequested) (Class|WidgetInteractionComponent|IsOverInteractableWidget (Variables|Default|GetWidgetInteraction))) (Variables|Default|GetInteractionAnimReady) (Variables|/Game/UI/WidgetBlueprints/WBP_Crosshair.WBP_Crosshair_C|GetCrosshairAllowed _crosshairref) (Variables|/Game/UI/WidgetBlueprints/WBP_Crosshair.WBP_Crosshair_C|GetStartFadeFinished _crosshairref)))
      (Utilities|FlowControl|Sequence
        (:then_0
          (Utilities|IsValid _interactref
            (:Is%20Valid
              (Default|SetInteractVisible _interactref (LocalVariables|GetFinalInteractionVisible%20%28Local%29)))))
        (:then_1
          (Default|SetCrosshairHovered (Variables|Default|GetCrosshairRef) (LocalVariables|GetFinalInteractionVisible%20%28Local%29)))))))