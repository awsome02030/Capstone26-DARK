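; BP_Keypad is an interactable keypad that takes over the player's view and movement during interaction.
; StopPlayer halts the character, ignores move input and uses a timeline to lerp control rotation toward LookAtPoint along the shortest path.
; EndKeypadInteraction restores move input.
; Helper events enable query-and-physics collision on supplied boxes (ToggleKeypads only enables) and swap the mesh material.
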(event `Toggle Keypads`
  (params (`Collision Boxes` :type "PrimitiveComponent Object Reference"))
  ; Toggle Keypad Collision Boxes
  (`PrimitiveComponent.SetCollisionEnabled` `Collision Boxes` "QueryAndPhysics"))

(event `Set Keypad Material`
  (params (`New Material` :type "MaterialInterface Object Reference"))
  ; Set Keypad Material
  (`PrimitiveComponent.SetMaterial` (`self.StaticMeshComponent`) 0 `New Material`))

(event `Stop Player`
  (bind _returnvalue (`GameplayStatics.GetPlayerController` 0))
  ; On interaction with keypad, make player look at LookAtPoint
  (`MovementComponent.StopMovementImmediately` (`Character.CharacterMovement` (`GameplayStatics.GetPlayerCharacter` 0)))
  (`Controller.SetIgnoreMoveInput` _returnvalue true)
  (set `self.Look Start Location` (`Controller.GetControlRotation` _returnvalue))
  (set `self.Look Target Location` (`KismetMathLibrary.FindLookAtRotation` (`PlayerCameraManager.GetCameraLocation` (`GameplayStatics.GetPlayerCameraManager` 0)) (`SceneComponent.K2_GetComponentLocation` (`self.LookAtPoint`))))
  (bind (_direction _lookat) (`Timeline|KeypadLookAnim`)
    (:`Update`
      (`Controller.SetControlRotation` _returnvalue (`KismetMathLibrary.RLerp` (`self.Look Start Location`) (`self.Look Target Location`) _lookat true)))))

(event `End Keypad Interaction`
  ; On interaction with keypad, make player look at LookAtPoint
  (`Controller.ResetIgnoreMoveInput` (`GameplayStatics.GetPlayerController` 0)))

(fn `UserConstructionScript`)